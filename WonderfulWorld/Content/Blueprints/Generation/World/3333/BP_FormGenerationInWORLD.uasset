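; Generates a blocky, voxel-style terrain of grass-dirt blocks, built from both the construction script and BeginPlay.
; AddChunk loops over a 3D grid and spawns a BP_BlockGrassDirt actor per cell, offsetting height by a rounded product of sines to form stepped hills.
; Player-based chunk tracking and removal helpers exist but are never called, and the instanced-mesh variants are disconnected.
; Tick prints the last computed block height for debugging.
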(event EventBeginPlay
  (CallFunction|AddChunk))

(event EventTick
  (params (DeltaSeconds :type Float%20%28single-precision%29))
  (Development|PrintString (Utilities|String|ToString(Float) (Variables|Default|Grass|Info|Getlowest%20point%20grass)) true true "(R=0.000000,G=0.660000,B=1.000000,A=1.000000)" 0.0))

(fn ConstructionScript
  (CallFunction|AddChunk))

(fn Ititialize
  (bind _output_get (Variables|Old|SetChunkSize (* (Variables|Settings|GetChunkLineElements) (Variables|Settings|GetVoxelSize))))
  (Variables|Old|SetChunkSizeHalf (/ _output_get 1)))

(fn UpdatePosition
  (bind _chunksizehalf (Variables|Old|GetChunkSizeHalf))
  (bind _returnvalue (Math|Conversions|ToFloat(Integer) _chunksizehalf))
  (bind _output_get (Variables|Old|SetCharacterPosition (* (Transformation|GetActorLocation (Game|Player|GetPlayerPawn 0)) "1.000000,1.000000, 0")))
  (if (or (!= (Variables|Old|GetChunkX) (Math|Float|Floor (/ (.X (Math|Vector|BreakVector _output_get)) _returnvalue))) (!= (Math|Float|Floor (/ (.Y (Math|Vector|BreakVector _output_get)) _returnvalue)) (Variables|Old|GetChunkY)))
    (Variables|Old|SetChunkX (Math|Float|Floor (/ (.X (Math|Vector|BreakVector _output_get)) _returnvalue)))
    (Variables|Old|SetChunkY (Math|Float|Floor (/ (.Y (Math|Vector|BreakVector _output_get)) _returnvalue)))
    (return true)
    (else
      (return false))))

(fn AddChunk
  (bind _frequence_grass (Variables|Default|Grass|GetFrequence%20Grass))
  (Utilities|FlowControl|Sequence
    (:then_0
      (for _index (range 1 (Variables|Default|Grass|GetLenght%20Grass)) ; x
        (for _index_2 (range 1 (Variables|Default|Grass|GetWidth%20Grass)) ; Y
          (for _index_3 (range 1 (Variables|Default|Grass|GetZ%20Grass)) ; Y
            (bind _output_get (Variables|Default|Grass|Info|Setlowest%20point%20grass (+ (Utilities|MultiplicationTileSize _index_3) (Math|Conversions|ToFloat(Integer) (* (Math|Float|Round (* (Math|Trig|Sin(Degrees) (* _index _frequence_grass)) (Math|Trig|Sin(Degrees) (* _index_2 _frequence_grass)) (Variables|Default|Grass|GetHeight%20Grass))) (Variables|Default|GetTile%20Size))))))
            (Game|SpawnActorfromClass "/Game/Blueprints/Generation/World/Blocks/BP_BlockGrassDirt.BP_BlockGrassDirt_C" (Math|Conversions|ToTransform(Vector) (Math|Vector|MakeVector (Utilities|MultiplicationTileSize _index) (Utilities|MultiplicationTileSize _index_2) _output_get)) "AlwaysSpawn" 0 0)))))))

(fn RemoveChunks
  (bind _chunksize (Variables|Old|GetChunkSize))
  (bind _chunksizehalf (Variables|Old|GetChunkSizeHalf))
  (bind _returnvalue (Math|Conversions|ToFloat(Integer) _chunksizehalf))
  (for (_array_element _array_index) 0
    (if (not (Utilities|CheckRadius (+ (* _chunksize (.X (Math|Vector2D|BreakVector2D _array_element))) _returnvalue) (+ (* _chunksize (.Y (Math|Vector2D|BreakVector2D _array_element))) _returnvalue)))
      (Actor|DestroyActor (Utilities|Array|Get(acopy) (Variables|Old|GetChunks) _array_index)))))