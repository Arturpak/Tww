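; Block terrain generator actor that builds a grid of block actors, with a box component sized in the construction script.
; GenereationChunks and DestroyChunks clear existing blocks, and generation calls AddChunk when its validity check finds none.
; AddChunk sums three sine-product layers for height, spawning one block class below zero and another otherwise.
; CheckBlock refreshes grass-dirt blocks; player-based chunk streaming helpers exist but are uncalled and incomplete.
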(event Custom|Destroy%20Chunks
  (bind _outactors (Actor|GetAllActorsOfClass "/Game/Blueprints/Generation/World/Blocks/BP_BlockDefault.BP_BlockDefault_C"))
  (for _array_element _outactors
    (Actor|DestroyActor _array_element))
  (Utilities|IsValid _array_element
    (:Is%20Valid
      (CallFunction|PrintText "Блоки удалены" "(R=1.000000,G=0.093059,B=0.072272,A=1.000000)" 2.0))
    (:Is%20Not%20Valid
      (CallFunction|PrintText "Отсутствуют блоки" "(R=1.000000,G=0.093059,B=0.072272,A=1.000000)" 2.0))))

(event Custom|Genereation%20Chunks
  (bind _outactors (Actor|GetAllActorsOfClass "/Game/Blueprints/Generation/World/Blocks/BP_BlockDefault.BP_BlockDefault_C"))
  (for _array_element _outactors
    (Actor|DestroyActor _array_element))
  (Utilities|IsValid _array_element
    (:Is%20Valid
      (CallFunction|PrintText "Отсутствуют блоки" "(R=1.000000,G=0.093059,B=0.072272,A=1.000000)" 2.0))
    (:Is%20Not%20Valid
      (CallFunction|PrintText "Генерация  блоков" "(R=0.087833,G=0.437500,B=0.062471,A=1.000000)" 2.0)
      (CallFunction|AddChunk))))

(event Custom|CheckBlock
  (bind _outactors (Actor|GetAllActorsOfClass "/Game/Blueprints/Generation/World/Blocks/BP_BlockGrassDirt.BP_BlockGrassDirt_C"))
  (for _array_element _outactors
    (Default|CheckBlock _array_element)))

(fn ConstructionScript
  (Components|Box|SetBoxExtent (Variables|Default|GetBox) (Math|Vector|MakeVector (Math|Conversions|ToFloat(Integer) (* (Variables|Default|Grass|GetLenght) 50)) (Math|Conversions|ToFloat(Integer) (* (Variables|Default|Grass|GetWidth%20) 50)) (Math|Conversions|ToFloat(Integer) (* (Math|Float|Ceil (+ (Variables|Default|Grass|GetFrequence%20Grass) (Variables|Default|Ground|GetFrequence%20Ground) (Variables|Default|Rock|GetFrequence%20Rock))) 50))) true)
  (Transformation|SetWorldLocation (Variables|Default|GetBox) (Math|Vector|MakeVector (Math|Conversions|ToFloat(Integer) (+ (* (Variables|Default|Grass|GetLenght) 50) 50)) (Math|Conversions|ToFloat(Integer) (+ (* (Variables|Default|Grass|GetWidth%20) 50) 50)) (Math|Conversions|ToFloat(Integer) (- (* (Math|Float|Ceil (+ (Variables|Default|Grass|GetFrequence%20Grass) (Variables|Default|Ground|GetFrequence%20Ground) (Variables|Default|Rock|GetFrequence%20Rock))) 50) 50))) false false))

(fn Ititialize
  (bind _output_get (Variables|Old|SetChunkSize (* (Variables|Settings|GetChunkLineElements) (Variables|Settings|GetVoxelSize))))
  (Variables|Old|SetChunkSizeHalf (/ _output_get 1)))

(fn UpdatePosition
  (bind _chunksizehalf (Variables|Old|GetChunkSizeHalf))
  (bind _returnvalue (Math|Conversions|ToFloat(Integer) _chunksizehalf))
  (bind _output_get (Variables|Old|SetCharacterPosition (* (Transformation|GetActorLocation (Game|Player|GetPlayerPawn 0)) "1.000000,1.000000, 0")))
  (if (or (!= (Variables|Old|GetChunkX) (Math|Float|Floor (/ (.X (Math|Vector|BreakVector _output_get)) _returnvalue))) (!= (Math|Float|Floor (/ (.Y (Math|Vector|BreakVector _output_get)) _returnvalue)) (Variables|Old|GetChunkY)))
    (Variables|Old|SetChunkX (Math|Float|Floor (/ (.X (Math|Vector|BreakVector _output_get)) _returnvalue)))
    (Variables|Old|SetChunkY (Math|Float|Floor (/ (.Y (Math|Vector|BreakVector _output_get)) _returnvalue)))
    (return true)
    (else
      (return false))))

(fn AddChunk
  (bind _frequence_rock (Variables|Default|Rock|GetFrequence%20Rock))
  (bind _frequence_ground (Variables|Default|Ground|GetFrequence%20Ground))
  (bind _frequence_grass (Variables|Default|Grass|GetFrequence%20Grass))
  (for _index (range 1 (Variables|Default|Grass|GetLenght)) ; x
    (for _index_2 (range 1 (Variables|Default|Grass|GetWidth%20)) ; Y
      (if (< (Math|Conversions|ToFloat(Integer) (* (Math|Float|Round (+ (* (Math|Trig|Sin(Degrees) (* _index _frequence_grass)) (Math|Trig|Sin(Degrees) (* _index_2 _frequence_grass)) (Variables|Default|Grass|GetHeight%20Grass)) (* (Math|Trig|Sin(Degrees) (* (* _index _frequence_ground) 0.7)) (Math|Trig|Sin(Degrees) (* _index_2 _frequence_ground)) (Variables|Default|Ground|GetHeight%20Ground)) (* (Math|Trig|Sin(Degrees) (* _index _frequence_rock)) (Math|Trig|Sin(Degrees) (* (* _index_2 _frequence_rock) 0.7)) (Variables|Default|Rock|GetHeight%20Rock)))) (Variables|Default|GetTile%20Size))) 0.0)
        (Utilities|SetBlockTESTER (Variables|Default|GetDirtBlock) true (Utilities|Array|Get(acopy) (Variables|Default|GetBP_BlockDefault)) (Math|Conversions|ToTransform(Vector) (Math|Vector|MakeVector (Utilities|MultiplicationTileSize _index) (Utilities|MultiplicationTileSize _index_2) (Math|Conversions|ToFloat(Integer) (* (Math|Float|Round (+ (* (Math|Trig|Sin(Degrees) (* _index _frequence_grass)) (Math|Trig|Sin(Degrees) (* _index_2 _frequence_grass)) (Variables|Default|Grass|GetHeight%20Grass)) (* (Math|Trig|Sin(Degrees) (* (* _index _frequence_ground) 0.7)) (Math|Trig|Sin(Degrees) (* _index_2 _frequence_ground)) (Variables|Default|Ground|GetHeight%20Ground)) (* (Math|Trig|Sin(Degrees) (* _index _frequence_rock)) (Math|Trig|Sin(Degrees) (* (* _index_2 _frequence_rock) 0.7)) (Variables|Default|Rock|GetHeight%20Rock)))) (Variables|Default|GetTile%20Size))))))
        (else
          (Utilities|SetBlockTESTER (Variables|Default|GetGrassBlock) true (Utilities|Array|Get(acopy) (Variables|Default|GetBP_BlockDefault) 1) (Math|Conversions|ToTransform(Vector) (Math|Vector|MakeVector (Utilities|MultiplicationTileSize _index) (Utilities|MultiplicationTileSize _index_2) (Math|Conversions|ToFloat(Integer) (* (Math|Float|Round (+ (* (Math|Trig|Sin(Degrees) (* _index _frequence_grass)) (Math|Trig|Sin(Degrees) (* _index_2 _frequence_grass)) (Variables|Default|Grass|GetHeight%20Grass)) (* (Math|Trig|Sin(Degrees) (* (* _index _frequence_ground) 0.7)) (Math|Trig|Sin(Degrees) (* _index_2 _frequence_ground)) (Variables|Default|Ground|GetHeight%20Ground)) (* (Math|Trig|Sin(Degrees) (* _index _frequence_rock)) (Math|Trig|Sin(Degrees) (* (* _index_2 _frequence_rock) 0.7)) (Variables|Default|Rock|GetHeight%20Rock)))) (Variables|Default|GetTile%20Size)))))))))))

(fn RemoveChunks
  (bind _chunksize (Variables|Old|GetChunkSize))
  (bind _chunksizehalf (Variables|Old|GetChunkSizeHalf))
  (bind _returnvalue (Math|Conversions|ToFloat(Integer) _chunksizehalf))
  (for (_array_element _array_index) 0
    (if (not (Utilities|CheckRadius (+ (* _chunksize (.X (Math|Vector2D|BreakVector2D _array_element))) _returnvalue) (+ (* _chunksize (.Y (Math|Vector2D|BreakVector2D _array_element))) _returnvalue)))
      (Actor|DestroyActor (Utilities|Array|Get(acopy) (Variables|Old|GetChunks) _array_index)))))