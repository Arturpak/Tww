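; World generation actor that streams a grid of BP_BlockDefault chunks around the player.
; Each tick it updates the player's chunk cell, removes chunks failing CheckRadius and spawns missing ones within RenderRange, tracked in parallel coordinate and actor arrays.
; The construction script also runs AddChunk.
; CheckRadius's distance test is left unconnected, and ChunkSizeHalf equals the full chunk size (divides by 1).
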(event EventBeginPlay
  (CallFunction|Ititialize))

(event EventTick
  (params (DeltaSeconds :type Float%20%28single-precision%29))
  (CallFunction|UpdatePosition)
  (CallFunction|RemoveChunks)
  (CallFunction|AddChunk))

(fn ConstructionScript
  (CallFunction|AddChunk))

(fn Ititialize
  (bind _output_get (Variables|Default|SetChunkSize (* (Variables|Settings|GetChunkLineElements) (Variables|Settings|GetVoxelSize))))
  (Variables|Default|SetChunkSizeHalf (/ _output_get 1)))

(fn UpdatePosition
  (bind _chunksizehalf (Variables|Default|GetChunkSizeHalf))
  (bind _returnvalue (Math|Conversions|ToFloat(Integer) _chunksizehalf))
  (bind _output_get (Variables|Default|SetCharacterPosition (* (Transformation|GetActorLocation (Game|Player|GetPlayerPawn 0)) "1.000000,1.000000, 0")))
  (if (or (!= (Variables|Default|GetChunkX) (Math|Float|Floor (/ (.X (Math|Vector|BreakVector _output_get)) _returnvalue))) (!= (Math|Float|Floor (/ (.Y (Math|Vector|BreakVector _output_get)) _returnvalue)) (Variables|Default|GetChunkY)))
    (Variables|Default|SetChunkX (Math|Float|Floor (/ (.X (Math|Vector|BreakVector _output_get)) _returnvalue)))
    (Variables|Default|SetChunkY (Math|Float|Floor (/ (.Y (Math|Vector|BreakVector _output_get)) _returnvalue)))
    (return true)
    (else
      (return false))))

(fn AddChunk
  (bind _chunksizehalf (Variables|Default|GetChunkSizeHalf))
  (bind _chunksize (Variables|Default|GetChunkSize))
  (bind _renderrange (Variables|Settings|GetRenderRange))
  (bind _chunkscoords (Variables|Default|GetChunksCoords))
  (bind _returnvalue (Math|Conversions|ToFloat(Integer) _chunksize))
  (bind _returnvalue_2 (Math|Conversions|ToFloat(Integer) _chunksizehalf))
  (bind _returnvalue_3 (* _renderrange -1))
  (for _index (range _returnvalue_3 _renderrange) ; x
    (for _index_2 (range _returnvalue_3 _renderrange) ; Y
      (if (Utilities|CheckRadius (+ (* (+ _index (Variables|Default|GetChunkX)) _returnvalue) _returnvalue_2) (+ (* (+ _index_2 (Variables|Default|GetChunkY)) _returnvalue) _returnvalue_2))
        (if (not (Utilities|Array|ContainsItem _chunkscoords (Math|Vector2D|MakeVector2D (Math|Conversions|ToFloat(Integer) (+ _index (Variables|Default|GetChunkX))) (Math|Conversions|ToFloat(Integer) (+ _index_2 (Variables|Default|GetChunkY))))))
          (Utilities|Array|Add _chunkscoords (Math|Vector2D|MakeVector2D (Math|Conversions|ToFloat(Integer) (+ _index (Variables|Default|GetChunkX))) (Math|Conversions|ToFloat(Integer) (+ _index_2 (Variables|Default|GetChunkY)))))
          (bind _returnvalue_4 (Game|SpawnActorfromClass "/Game/Blueprints/Generation/World/Blocks/BP_BlockDefault.BP_BlockDefault_C" (Math|Conversions|ToTransform(Vector) (Math|Vector|MakeVector (* (+ _index (Variables|Default|GetChunkX)) _returnvalue) (* (+ _index_2 (Variables|Default|GetChunkY)) _returnvalue) 4.0)) "Undefined" 0 0))
          (Utilities|Array|Add (Variables|Default|GetChunks) _returnvalue_4))))))

(fn RemoveChunks
  (bind _chunksize (Variables|Default|GetChunkSize))
  (bind _chunksizehalf (Variables|Default|GetChunkSizeHalf))
  (bind _returnvalue (Math|Conversions|ToFloat(Integer) _chunksizehalf))
  (for (_array_element _array_index) (Variables|Default|GetChunksCoords)
    (if (not (Utilities|CheckRadius (+ (* _chunksize (.X (Math|Vector2D|BreakVector2D _array_element))) _returnvalue) (+ (* _chunksize (.Y (Math|Vector2D|BreakVector2D _array_element))) _returnvalue)))
      (Actor|DestroyActor (Utilities|Array|Get(acopy) (Variables|Default|GetChunks) _array_index))
      (Utilities|Array|RemoveIndex (Variables|Default|GetChunksCoords) _array_index)
      (Utilities|Array|RemoveIndex (Variables|Default|GetChunks) _array_index))))