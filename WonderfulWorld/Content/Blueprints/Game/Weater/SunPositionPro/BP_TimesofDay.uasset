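; Time-of-day controller that animates the sun by pitching a DirectionalLight every Tick at a set speed while UpdateSun is on.
; Ctrl+1 toggles that motion; when it is off, holding Up or Down nudges the pitch through looping timers.
; Preset events store the light rotation with name and slot in an in-memory struct array and restore it by index; the separate Save event only adds placeholder data.
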(event EventTick
  (params (DeltaSeconds :type Float%20%28single-precision%29))
  (CallFunction|RotationSun))

(event Input|KeyboardEvents|Down
  (params (Key :type Key%20Structure))
  (:Pressed
    (bind _returnvalue (Utilities|Time|SetTimerbyFunctionName 0 "Sun-" 0.01 true))
    (bind _output_get (Variables|Default|PlayerConnect|SetV-Sun- _returnvalue)))
  (:Released
    (Utilities|Time|ClearandInvalidateTimerbyHandle _output_get)))

(event Input|KeyboardEvents|Ctrl1
  (params (Key :type Key%20Structure))
  (:Pressed
    (if (Variables|Default|Settings|GetUpdateSun)
      (Variables|Default|Settings|SetUpdateSun false)
      (else
        (Variables|Default|Settings|SetUpdateSun true)))))

(event Input|KeyboardEvents|Up
  (params (Key :type Key%20Structure))
  (:Pressed
    (bind _returnvalue (Utilities|Time|SetTimerbyFunctionName 0 "Sun+" 0.01 true))
    (bind _output_get (Variables|Default|PlayerConnect|SetV_Sun+ _returnvalue)))
  (:Released
    (Utilities|Time|ClearandInvalidateTimerbyHandle _output_get)))

(event Custom|Load%20Slot
  (bind _slots_load (Variables|Default|GetSlots%20Load))
  (bind _timeofdaysave (Variables|Default|Presset|GetTimeOfDaySave))
  (bind _output (Utilities|Array|Get(acopy) _timeofdaysave _slots_load))
  (bind (_namesave _positionsun _slots) (Utilities|Struct|BreakS_TimeOfDaySave _output))
  (Transformation|SetWorldRotation (Variables|/Script/Engine.Light|GetLightComponent (Variables|Default|Settings|GetDirectional%20light)) _positionsun false false)
  (bind _output_get (Variables|Default|Presset|Save|SetName%20Save _namesave))
  (bind _output_get_2 (Variables|Default|Presset|Save|SetSlots%20Save _slots))
  (CallFunction|PrintText (Utilities|String|ToString(Text) (Utilities|Text|FormatText "Загружено 
Slots - {A} 
Name - {B} 
Rotation - {C}" _output_get_2 _output_get (Utilities|Text|ToText(String) _positionsun))) "(R=1.000000,G=0.339252,B=0.087070,A=1.000000)" 8.0))

(event Custom|Save%20Atmosphere
  (bind _output_get (Variables|Default|SetDirLightRotation (Transformation|GetActorRotation (Variables|Default|Settings|GetDirectional%20light))))
  (Variables|Default|SetTimeOfDay (Utilities|Struct|MakeS_TimeOfDaySave (Variables|Default|Presset|Save|GetName%20Save) _output_get (Variables|Default|Presset|Save|GetSlots%20Save)))
  (Utilities|Array|AddUnique (Variables|Default|Presset|GetTimeOfDaySave) (Variables|Default|GetTimeOfDay)))

(event Custom|Save
  (Utilities|Map|Add :TargetMap (Variables|Default|Get2321321) :Key "ывывывы"))

(fn ConstructionScript)

(fn RotationSun
  (if (Variables|Default|Settings|GetUpdateSun)
    (Transformation|AddActorLocalRotation (Variables|Default|Settings|GetDirectional%20light) (Math|Rotator|MakeRotator 0.0 (* (Utilities|Time|GetWorldDeltaSeconds) (Variables|Default|Settings|GetSpeed)) 0.0) false false)))

(fn DefaultConnect
  (params (InUpdateSun :type Boolean))
  (bind _output_get (Variables|Default|Settings|SetUpdateSun InUpdateSun))
  (return 0 _output_get))

(fn Sun+
  (if (not (Variables|Default|Settings|GetUpdateSun))
    (Transformation|AddActorLocalRotation (Variables|Default|Settings|GetDirectional%20light) (Math|Rotator|MakeRotator 0.0 0.1 0.0) false false)))

(fn Sun-
  (if (not (Variables|Default|Settings|GetUpdateSun))
    (Transformation|AddActorLocalRotation (Variables|Default|Settings|GetDirectional%20light) (Math|Rotator|MakeRotator 0.0 -0.1 0.0) false false)))