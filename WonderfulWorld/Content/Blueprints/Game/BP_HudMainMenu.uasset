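; Main menu HUD Blueprint that shows or hides the W_MainMenu widget through the DisplayMainMenu event.
; Showing creates the widget if none is valid, adds it to the viewport, and gives player 0 Game and UI input focused on it with the mouse cursor visible.
; Hiding removes and clears a valid widget and hides the cursor, but leaves the input mode unchanged.
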(event Custom|DisplayMainMenu
  (params (Visible? :type Boolean))
  (if Visible?
    (Variables|Default|GetW_MainMenu
      (:then
        _)
      (:else
        (bind _returnvalue (UserInterface|CreateWidget "/Game/Blueprints/Interface/MainMenu/W_MainMenu.W_MainMenu_C" (Game|GetPlayerController 0)))
        (bind _output_get (Variables|Default|SetW_MainMenu _returnvalue))))
    (UserInterface|Viewport|AddtoViewport _output_get 0)
    (Input|SetInputModeGameandUI (Game|GetPlayerController 0) _output_get "DoNotLock" true)
    (Variables|/Script/Engine.PlayerController|SetbShowMouseCursor (Game|GetPlayerController 0) true)
    (else
      (bind _w_mainmenu (Variables|Default|GetW_MainMenu)
        (:then
          (Widget|RemovefromParent _w_mainmenu)
          (Variables|Default|SetW_MainMenu 0)
          (Variables|/Script/Engine.PlayerController|SetbShowMouseCursor (Game|GetPlayerController 0) false))
        (:else)))))

(fn ConstructionScript)