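; Player controller Blueprint that sets game-only input on BeginPlay and handles the keys that toggle two HUD displays.
; Tab toggles the ControlWorld display and X toggles the game menu, both through display functions on the HUD.
; Each toggle infers the open state from whether the HUD's corresponding reference is valid, so the controller keeps no state of its own.
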(event EventBeginPlay
  (Input|SetInputModeGameOnly self))

(event Input|KeyboardEvents|X
  (params (Key :type Key%20Structure :default "None"))
  (bind _hud (CallFunction|GetHUD))
  (:Pressed
    (Utilities|IsValid (Variables|/Game/Blueprints/Game/BP_HUD.BP_HUD_C|GetW_GameMenu _hud)
      (:Is%20Valid
        (Default|DisplayGameMenu _hud false))
      (:Is%20Not%20Valid
        (Default|DisplayGameMenu _hud true)))))

(event Input|KeyboardEvents|Tab
  (params (Key :type Key%20Structure :default "None"))
  (bind _hud (CallFunction|GetHUD))
  (:Pressed
    (Utilities|IsValid (Variables|/Game/Blueprints/Game/BP_HUD.BP_HUD_C|GetControlWorld (CallFunction|GetHUD))
      (:Is%20Valid
        (Default|DisplayControlWorld _hud false))
      (:Is%20Not%20Valid
        (Default|DisplayControlWorld _hud true)))))

(fn ConstructionScript)