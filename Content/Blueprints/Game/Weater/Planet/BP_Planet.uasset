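; BP_Planet is a planet actor that spins continuously around its pitch axis at a configurable Speed.
; Tick applies the frame-rate-independent rotation and also creates and stores a new dynamic instance of M_Planet_Inst on its mesh every frame.
; A timeline driving the material's Max parameter and a Light Direction setter are disconnected.
; NewFunction0 repeats the rotation behind an UpdatePlanet flag but is not called here.
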(event EventTick
  (params (DeltaSeconds :type Float%20%28single-precision%29))
  (Transformation|AddActorLocalRotation self (Math|Rotator|MakeRotator 0.0 (* (Utilities|Time|GetWorldDeltaSeconds) (Variables|Default|GetSpeed)) 0.0) false false)
  (bind _returnvalue (Rendering|Material|CreateDynamicMaterialInstance (Variables|Default|GetStaticMesh) 0 "/Game/Blueprints/Game/Weater/Planet/M_Planet_Inst.M_Planet_Inst" "Max" :!class /Script/Engine.PrimitiveComponent))
  (bind _output_get (Variables|Default|SetMaterialInstance _returnvalue)))

(fn ConstructionScript)

(fn NewFunction0
  (if (Variables|Default|GetUpdate%20Planet)
    (Transformation|AddActorLocalRotation (Math|Rotator|MakeRotator 0.0 (* (Utilities|Time|GetWorldDeltaSeconds) (Variables|Default|GetSpeed)) 0.0) false false)))