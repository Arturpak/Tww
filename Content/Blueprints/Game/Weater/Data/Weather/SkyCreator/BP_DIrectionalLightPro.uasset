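; BP_DIrectionalLightPro is a sky-lighting Blueprint that configures a star dome and keeps a moon light positioned relative to its own rotation.
; The construction script sets the sky dome's visibility from the VisibleStars flag.
; When a DIrectionalMoon reference is valid, it rotates that light to face roughly opposite this actor, with flipped yaw and an inverted, offset pitch.
; The event graph holds no active logic.
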(event EventBeginPlay)

(event EventTick
  (params (DeltaSeconds :type Float%20%28single-precision%29)))

(fn ConstructionScript
  (bind _returnvalue (Transformation|GetActorRotation))
  (bind (_roll _pitch _yaw) (Math|Rotator|BreakRotator _returnvalue))
  (Utilities|FlowControl|Sequence
    (:then_1
      (Rendering|SetVisibility (Variables|Default|GetBP_SkyDome) (Variables|Default|GetVisibleStars) false))
    (:then_2
      (Utilities|IsValid (Variables|Default|GetDIrectionalMoon)
        (:Is%20Valid
          (Transformation|SetWorldRotation (Variables|/Script/Engine.Actor|GetRootComponent (Variables|Default|GetDIrectionalMoon)) (Math|Rotator|MakeRotator _roll (* (+ _pitch 15.0) -1.0) (+ _yaw 1.8e+02)) false false))))
    (:then_3)
    (:then_4)))