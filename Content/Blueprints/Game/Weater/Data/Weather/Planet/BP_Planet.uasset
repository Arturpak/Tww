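; BP_Planet is a planet actor in the weather content that orients a moon static mesh relative to its own rotation.
; The Construction Script sets the moon mesh's world rotation to the result of GetRotateSun with a factor of 2.
; GetRotateSun scales each component of the actor's rotation by that factor, so the moon's angles are double the actor's whenever construction runs.
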(fn ConstructionScript
  (Transformation|SetWorldRotation (Variables|Default|GetMoonStaticMesh) (CallFunction|GetRotateSun 2.0) false false))

(fn GetRotateSun
  (params (B :type Float%20%28single-precision%29))
  (bind _self self)
  (bind _returnvalue (Transformation|GetActorRotation _self))
  (bind (_roll _pitch _yaw) (Math|Rotator|BreakRotator _returnvalue))
  (return (Math|Rotator|MakeRotator (* _roll B) (* _pitch B) (* _yaw B))))