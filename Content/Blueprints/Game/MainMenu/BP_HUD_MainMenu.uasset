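; BP_HUD_MainMenu is the main menu HUD Blueprint that shows or hides the W_MainMenu widget through its DisplayMainMenu event.
; Showing creates the widget if none is valid, adds it to the viewport, then sets Game and UI input focused on it with a visible cursor.
; Hiding removes and clears a valid widget, restores Game Only input and hides the cursor.
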(event Custom|DisplayMainMenu
  (params (Condition :type Boolean))
  (bind _player_conroller_menu (CallFunction|PlayerConrollerMenu))
  (if Condition
    (Variables|Default|GetW_MainMenu
      (:then
        _)
      (:else
        (bind _returnvalue (UserInterface|CreateWidget "/Game/Blueprints/Game/MainMenu/Witgets/W_MainMenu.W_MainMenu_C" (CallFunction|PlayerConrollerMenu)))
        (bind _output_get (Variables|Default|SetW_MainMenu _returnvalue))))
    (UserInterface|Viewport|AddtoViewport _output_get 0)
    (Input|SetInputModeGameandUI _player_conroller_menu _output_get "DoNotLock" false)
    (Variables|/Script/Engine.PlayerController|SetbShowMouseCursor _player_conroller_menu true)
    (else
      (bind _w_mainmenu (Variables|Default|GetW_MainMenu)
        (:then
          (Widget|RemovefromParent _w_mainmenu)
          (Input|SetInputModeGameOnly (CallFunction|PlayerConrollerMenu))
          (Variables|Default|SetW_MainMenu 0)
          (Variables|/Script/Engine.PlayerController|SetbShowMouseCursor (CallFunction|PlayerConrollerMenu) false))
        (:else)))))

(fn ConstructionScript)