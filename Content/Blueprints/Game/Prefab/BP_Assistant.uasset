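; BP_Assistant is a shared helper that provides quick access to common game objects and a text printing utility.
; Its getters fetch player index 0's HUD and character plus the game instance, cast to BP_HUD, FirstPersonCharacter and BP_GameInstance.
; A failed cast stops the getter before it reaches its return.
; Print Text wraps PrintString, exposing only the string, color and duration.
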(fn GetHUD
  (bind _asbp_hud (Utilities|Casting|CastToBP_HUD (HUD|GetHUD (Game|GetPlayerController 0))))
  (return _asbp_hud))

(fn GetPlayer
  (bind _asfirst_person_character (Utilities|Casting|CastToFirstPersonCharacter (Game|GetPlayerCharacter 0)))
  (return _asfirst_person_character))

(fn PrintText
  (params (InString :type String) (TextColor :type Linear%20Color%20Structure :default "(R=1.000000,G=0.339252,B=0.087070,A=1.000000)") (Duration :type Float%20%28single-precision%29))
  (Development|PrintString 0 InString true true TextColor Duration))

(fn GameInstance
  (bind _asbp_game_instance (Utilities|Casting|CastToBP_GameInstance (Game|GetGameInstance)))
  (return _asbp_game_instance))