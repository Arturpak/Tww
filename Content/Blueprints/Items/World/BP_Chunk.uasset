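; BP_Chunk is a world chunk actor that builds a 3D grid of tiles and displays its own location as floating text.
; When Visible, CreateChunk fills an InstancedStaticMesh over symmetric X, Y and Z ranges spaced by TileSize.
; It runs in both the construction script and BeginPlay, without clearing earlier instances.
; UpdatePosition stores the actor location and writes it, scaled to metres, to a Text3D label every tick.
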(event EventBeginPlay
  (CallFunction|CreateChunk))

(event EventTick
  (params (DeltaSeconds :type Float%20%28single-precision%29))
  (CallFunction|UpdatePosition))

(fn ConstructionScript
  (CallFunction|CreateChunk)
  (CallFunction|UpdatePosition))

(fn CreateChunk
  (bind _x (Variables|Default|GetX))
  (bind _y (Variables|Default|GetY))
  (bind _z (Variables|Default|GetZ))
  (if (Variables|Default|GetVisible)
    (for _index (range (* _x -1) _x) ; x
      (LocalVariables|SetL_X _index)
      (for _index_2 (range (* _y -1) _y) ; Y
        (LocalVariables|SetL_Y _index_2)
        (for _index_3 (range (* _z -1) _z) ; Y
          (LocalVariables|SetL_Z _index_3)
          (Components|InstancedStaticMesh|AddInstance (Variables|Default|GetInstancedStaticMesh) (Math|Conversions|ToTransform(Vector) (Math|Vector|MakeVector (Math|Conversions|ToFloat(Integer) (* (LocalVariables|GetL_X) (Variables|Default|GetTile%20Size))) (Math|Conversions|ToFloat(Integer) (* (LocalVariables|GetL_Y) (Variables|Default|GetTile%20Size))) (Math|Conversions|ToFloat(Integer) (* (LocalVariables|GetL_Z) (Variables|Default|GetTile%20Size)))))))))))

(fn UpdatePosition
  (bind _self self)
  (bind _returnvalue (Transformation|GetActorLocation _self))
  (bind (_x _y _z) (Math|Vector|BreakVector _returnvalue))
  (Variables|Default|SetPositionChunk (Transformation|GetActorLocation self))
  (Class|Text3DComponent|SetText (Variables|Default|GetText3D) (Utilities|Text|FormatText "{A} 
{B}" self (Utilities|Text|ToText(String) (Utilities|String|Append (Utilities|String|ToString(Float) (/ _x 1e+02)) "  ||||||  " (Utilities|String|ToString(Float) (/ _y 1e+02)) "  ||||||  " (Utilities|String|ToString(Float) (/ _z 1e+02)))))))