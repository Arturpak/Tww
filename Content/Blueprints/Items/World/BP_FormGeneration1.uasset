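; BP_FormGeneration1 is a world actor that builds a blocky, rolling terrain from instanced static mesh tiles.
; AddChunk runs in both the construction script and BeginPlay, filling a Lenght by Width grid with heights from two multiplied sine waves, rounded to tile steps.
; Player-following chunk functions (Ititialize, UpdatePosition, RemoveChunks) are never called here, and CheckRadius's distance test is unwired.
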(event EventBeginPlay
  (CallFunction|AddChunk))

(fn ConstructionScript
  (CallFunction|AddChunk))

(fn Ititialize
  (bind _output_get (Variables|Default|SetChunkSize (* (Variables|Settings|GetChunkLineElements) (Variables|Settings|GetVoxelSize))))
  (Variables|Default|SetChunkSizeHalf (/ _output_get 1)))

(fn UpdatePosition
  (bind _chunksizehalf (Variables|Default|GetChunkSizeHalf))
  (bind _returnvalue (Math|Conversions|ToFloat(Integer) _chunksizehalf))
  (bind _output_get (Variables|Default|SetCharacterPosition (* (Transformation|GetActorLocation (Game|Player|GetPlayerPawn 0)) "1.000000,1.000000, 0")))
  (if (or (!= (Variables|Default|GetChunkX) (Math|Float|Floor (/ (.X (Math|Vector|BreakVector _output_get)) _returnvalue))) (!= (Math|Float|Floor (/ (.Y (Math|Vector|BreakVector _output_get)) _returnvalue)) (Variables|Default|GetChunkY)))
    (Variables|Default|SetChunkX (Math|Float|Floor (/ (.X (Math|Vector|BreakVector _output_get)) _returnvalue)))
    (Variables|Default|SetChunkY (Math|Float|Floor (/ (.Y (Math|Vector|BreakVector _output_get)) _returnvalue)))
    (return true)
    (else
      (return false))))

(fn AddChunk
  (bind _frequence (Variables|Default|GetFrequence))
  (bind _tilesize (Variables|Default|GetTileSize))
  (for _index (range 1 (Variables|Default|GetLenght)) ; x
    (for _index_2 (range 1 (Variables|Default|GetWidth)) ; Y
      (Components|InstancedStaticMesh|AddInstance (Variables|Default|GetInstancedStaticMesh) (Math|Conversions|ToTransform(Vector) (Math|Vector|MakeVector (Math|Conversions|ToFloat(Integer) (* _index _tilesize)) (Math|Conversions|ToFloat(Integer) (* _index_2 _tilesize)) (Math|Conversions|ToFloat(Integer) (* (Math|Float|Round (* (Math|Trig|Sin(Degrees) (* _index _frequence)) (Math|Trig|Sin(Degrees) (* _index_2 _frequence)) (Variables|Default|GetHeight))) (Variables|Default|GetTileSize)))))))))

(fn RemoveChunks
  (bind _chunksize (Variables|Default|GetChunkSize))
  (bind _chunksizehalf (Variables|Default|GetChunkSizeHalf))
  (bind _returnvalue (Math|Conversions|ToFloat(Integer) _chunksizehalf))
  (for (_array_element _array_index) (Variables|Default|GetChunksCoords)
    (if (not (Utilities|CheckRadius (+ (* _chunksize (.X (Math|Vector2D|BreakVector2D _array_element))) _returnvalue) (+ (* _chunksize (.Y (Math|Vector2D|BreakVector2D _array_element))) _returnvalue)))
      (Actor|DestroyActor (Utilities|Array|Get(acopy) (Variables|Default|GetChunks) _array_index))
      (Utilities|Array|RemoveIndex (Variables|Default|GetChunksCoords) _array_index)
      (Utilities|Array|RemoveIndex (Variables|Default|GetChunks) _array_index))))