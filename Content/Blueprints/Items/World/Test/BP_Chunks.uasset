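; Test chunk spawner that fills a grid around the player with BP_BlockNew actors to build a voxel-style world.
; Chunk size is derived from voxel size and elements per line on BeginPlay.
; Each Tick updates the player's chunk coordinate and scans the render range, spawning unrecorded chunks that pass CheckRadius, whose distance test appears unconnected.
; Coordinates and actors are stored to prevent duplicates, and none are removed.
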(event EventBeginPlay
  (CallFunction|Init))

(event EventTick
  (params (DeltaSeconds :type Float%20%28single-precision%29))
  (CallFunction|UpdatePosition)
  (CallFunction|AddChunk))

(fn ConstructionScript)

(fn UpdatePosition
  (bind _output_get (Variables|Default|SetCharacterPosition (* (Transformation|GetActorLocation (Game|Player|GetPlayerPawn 0)) "1.000000,1.000000,0.000000")))
  (if (or (!= (Variables|Default|GetChunkX) (Math|Float|Floor (/ (.X (Math|Vector|BreakVector _output_get)) (Math|Conversions|ToFloat(Integer) (Variables|Default|GetChunkSizeHalf))))) (!= (Variables|Default|GetChunkX) (Math|Float|Floor (/ (.Y (Math|Vector|BreakVector _output_get)) (Math|Conversions|ToFloat(Integer) (Variables|Default|GetChunkSizeHalf))))))
    (Variables|Default|SetChunkX (Math|Float|Floor (/ (.X (Math|Vector|BreakVector _output_get)) (Math|Conversions|ToFloat(Integer) (Variables|Default|GetChunkSizeHalf)))))
    (Variables|Default|SetChunkY (Math|Float|Floor (/ (.Y (Math|Vector|BreakVector _output_get)) (Math|Conversions|ToFloat(Integer) (Variables|Default|GetChunkSizeHalf)))))
    (return true)
    (else
      (return false))))

(fn Init
  (bind _output_get (Variables|Default|SetChunkSize (* (Variables|Settings|GetChunkLineElements) (Variables|Settings|GetVoxelSize))))
  (Variables|Default|SetChunkSizeHalf (/ _output_get 1)))

(fn AddChunk
  (bind _renderrange (Variables|Settings|GetRenderRange))
  (bind _chunkcoords (Variables|Default|GetChunkCoords))
  (bind _returnvalue (* _renderrange -1))
  (for _index (range _returnvalue _renderrange) ; Y
    (for _index_2 (range _returnvalue _renderrange) ; X
      (if (Utilities|CheckRadius (+ (* (+ _index_2 (Variables|Default|GetChunkX)) (Math|Conversions|ToFloat(Integer) (Variables|Default|GetChunkSize))) (Math|Conversions|ToFloat(Integer) (Variables|Default|GetChunkSizeHalf))) (+ (* (+ _index (Variables|Default|GetChunkY)) (Math|Conversions|ToFloat(Integer) (Variables|Default|GetChunkSize))) (Math|Conversions|ToFloat(Integer) (Variables|Default|GetChunkSizeHalf))))
        (if (not (Utilities|Array|ContainsItem _chunkcoords (Math|Vector2D|MakeVector2D (Math|Conversions|ToFloat(Integer) (+ _index_2 (Variables|Default|GetChunkX))) (Math|Conversions|ToFloat(Integer) (+ _index (Variables|Default|GetChunkY))))))
          (Utilities|Array|Add _chunkcoords (Math|Vector2D|MakeVector2D (Math|Conversions|ToFloat(Integer) (+ _index_2 (Variables|Default|GetChunkX))) (Math|Conversions|ToFloat(Integer) (+ _index (Variables|Default|GetChunkY)))))
          (bind _returnvalue_2 (Game|SpawnActorfromClass "/Game/Blueprints/Items/Blocks/BP_BlockNew.BP_BlockNew_C" (Math|Transform|MakeTransform (Math|Vector|MakeVector (* (+ _index_2 (Variables|Default|GetChunkX)) (Math|Conversions|ToFloat(Integer) (Variables|Default|GetChunkSize))) (* (+ _index (Variables|Default|GetChunkY)) (Math|Conversions|ToFloat(Integer) (Variables|Default|GetChunkSize))) 0.0)) "Undefined" 0 0))
          (Utilities|Array|Add (Variables|Default|GetChunk) _returnvalue_2))))))