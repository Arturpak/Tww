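; Procedural terrain generator actor that builds a voxel-style landscape of dirt and grass blocks in the construction script.
; The construction script resizes the Box and, when VIsibleBlock is set, runs AddChunk over a Lenght × Width × Height grid.
; Three summed sine-product waves offset each column, with mesh instances forming dirt and a grass top at non-negative height.
; Event graph events are empty or disconnected, and player-based chunk streaming helpers are never called here.
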(event Custom|Genereation%20Chunks)

(event Custom|CheckBlock)

(event Custom|Destroy%20Chunks)

(fn ConstructionScript
  (Components|Box|SetBoxExtent (Variables|Default|GetBox) (Math|Vector|MakeVector (Math|Conversions|ToFloat(Integer) (* (Variables|Default|GetLenght) 50)) (Math|Conversions|ToFloat(Integer) (* (Variables|Default|GetWidth%20) 50)) (Math|Conversions|ToFloat(Integer) (* (Math|Float|Ceil (+ (Variables|Default|Grass|GetFrequence%20Grass) (Variables|Default|Ground|GetFrequence%20Ground) (Variables|Default|Rock|GetFrequence%20Rock))) 50))) true)
  (Transformation|SetWorldLocation (Variables|Default|GetBox) (+ (Transformation|GetActorLocation) (Math|Vector|MakeVector (Math|Conversions|ToFloat(Integer) (+ (* (Variables|Default|GetLenght) 50) 50)) (Math|Conversions|ToFloat(Integer) (+ (* (Variables|Default|GetWidth%20) 50) 50)) (Math|Conversions|ToFloat(Integer) (- (* (Math|Float|Ceil (+ (Variables|Default|Grass|GetFrequence%20Grass) (Variables|Default|Ground|GetFrequence%20Ground) (Variables|Default|Rock|GetFrequence%20Rock))) 50) 50)))) false false)
  (if (Variables|Default|GetVIsible%20Block?)
    (CallFunction|AddChunk)))

(fn Ititialize
  (bind _output_get (Variables|Old|SetChunkSize (* (Variables|Settings|GetChunkLineElements) (Variables|Settings|GetVoxelSize))))
  (Variables|Old|SetChunkSizeHalf (/ _output_get 1)))

(fn UpdatePosition
  (bind _chunksizehalf (Variables|Old|GetChunkSizeHalf))
  (bind _returnvalue (Math|Conversions|ToFloat(Integer) _chunksizehalf))
  (bind _output_get (Variables|Old|SetCharacterPosition (* (Transformation|GetActorLocation (Game|Player|GetPlayerPawn 0)) "1.000000,1.000000, 0")))
  (if (or (!= (Variables|Old|GetChunkX) (Math|Float|Floor (/ (.X (Math|Vector|BreakVector _output_get)) _returnvalue))) (!= (Math|Float|Floor (/ (.Y (Math|Vector|BreakVector _output_get)) _returnvalue)) (Variables|Old|GetChunkY)))
    (Variables|Old|SetChunkX (Math|Float|Floor (/ (.X (Math|Vector|BreakVector _output_get)) _returnvalue)))
    (Variables|Old|SetChunkY (Math|Float|Floor (/ (.Y (Math|Vector|BreakVector _output_get)) _returnvalue)))
    (return true)
    (else
      (return false))))

(fn AddChunk
  (bind _frequence_rock (Variables|Default|Rock|GetFrequence%20Rock))
  (bind _height (Variables|Default|GetHeight))
  (bind _frequence_ground (Variables|Default|Ground|GetFrequence%20Ground))
  (bind _frequence_grass (Variables|Default|Grass|GetFrequence%20Grass))
  (for _index (range 1 (Variables|Default|GetLenght)) ; x
    (LocalVariables|SetL_X _index)
    (for _index_2 (range 1 (Variables|Default|GetWidth%20)) ; Y
      (LocalVariables|SetL_Y _index_2)
      (for _index_3 (range 0 _height) ; Y
        (bind _output_get (LocalVariables|SetL_Z _index_3))
        (LocalVariables|SetL_TransformBlock (Math|Conversions|ToTransform(Vector) (Math|Vector|MakeVector (Utilities|MultiplicationTileSize (LocalVariables|GetL_X)) (Utilities|MultiplicationTileSize (LocalVariables|GetL_Y)) (Math|Conversions|ToFloat(Integer) (+ (Math|Float|Truncate (Utilities|MultiplicationTileSize (LocalVariables|GetL_Z))) (* (Math|Float|Round (+ (* (Math|Trig|Sin(Degrees) (* (LocalVariables|GetL_X) _frequence_grass)) (Math|Trig|Sin(Degrees) (* (LocalVariables|GetL_Y) _frequence_grass)) (Variables|Default|Grass|GetHeight%20Grass)) (* (Math|Trig|Sin(Degrees) (* (* (LocalVariables|GetL_X) _frequence_ground) 0.7)) (Math|Trig|Sin(Degrees) (* (LocalVariables|GetL_Y) _frequence_ground)) (Variables|Default|Ground|GetHeight%20Ground)) (* (Math|Trig|Sin(Degrees) (* (LocalVariables|GetL_X) _frequence_rock)) (Math|Trig|Sin(Degrees) (* (* (LocalVariables|GetL_Y) _frequence_rock) 0.4)) (Variables|Default|Rock|GetHeight%20Rock)))) (Variables|Default|GetTile%20Size)) 0)))))
        (if (== _output_get _height)
          (if (< (Math|Conversions|ToFloat(Integer) (+ (Math|Float|Truncate (Utilities|MultiplicationTileSize (LocalVariables|GetL_Z))) (* (Math|Float|Round (+ (* (Math|Trig|Sin(Degrees) (* (LocalVariables|GetL_X) _frequence_grass)) (Math|Trig|Sin(Degrees) (* (LocalVariables|GetL_Y) _frequence_grass)) (Variables|Default|Grass|GetHeight%20Grass)) (* (Math|Trig|Sin(Degrees) (* (* (LocalVariables|GetL_X) _frequence_ground) 0.7)) (Math|Trig|Sin(Degrees) (* (LocalVariables|GetL_Y) _frequence_ground)) (Variables|Default|Ground|GetHeight%20Ground)) (* (Math|Trig|Sin(Degrees) (* (LocalVariables|GetL_X) _frequence_rock)) (Math|Trig|Sin(Degrees) (* (* (LocalVariables|GetL_Y) _frequence_rock) 0.4)) (Variables|Default|Rock|GetHeight%20Rock)))) (Variables|Default|GetTile%20Size)) 0)) 0.0)
            ;[0.4115 0.3056 0.1243] Location Block
            (Utilities|SetStatic/Actor (Variables|Default|GetDirtBlock) false (Utilities|SetBlock) (LocalVariables|GetL_TransformBlock) :!label _label)
            (else
              (Utilities|SetStatic/Actor (Variables|Default|GetGrassBlock) false (Utilities|SetBlock 1) (LocalVariables|GetL_TransformBlock))))
          (else
            (goto _label)))))))

(fn RemoveChunks
  (bind _chunksize (Variables|Old|GetChunkSize))
  (bind _chunksizehalf (Variables|Old|GetChunkSizeHalf))
  (bind _returnvalue (Math|Conversions|ToFloat(Integer) _chunksizehalf))
  (for (_array_element _array_index) 0
    (if (not (Utilities|CheckRadius (+ (* _chunksize (.X (Math|Vector2D|BreakVector2D _array_element))) _returnvalue) (+ (* _chunksize (.Y (Math|Vector2D|BreakVector2D _array_element))) _returnvalue)))
      (Actor|DestroyActor (Utilities|Array|Get(acopy) (Variables|Old|GetChunks) _array_index)))))