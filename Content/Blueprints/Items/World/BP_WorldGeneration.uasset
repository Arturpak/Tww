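; World generation actor that spawns a square grid of BP_Chunk actors around the world origin on BeginPlay.
; CreatesChunks loops X and Y across plus or minus RenderRange, spacing chunks by TileSize times 100, and records each position and actor in BlockCoordinates.
; Player-following logic (UpdatePosition, radius and duplicate checks) and the PrintInfo debug print are present but never run, so the grid stays static.
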(event EventTick
  (params (DeltaSeconds :type Float%20%28single-precision%29)))

(event EventBeginPlay
  (CallFunction|CreatesChunks))

(fn ConstructionScript)

(fn CreatesChunks
  (bind _renderrange (Variables|Settings|GetRenderRange))
  (bind _renderrange_2 (Variables|Settings|GetRenderRange))
  (for _index (range (* _renderrange_2 -1) _renderrange_2) ; x
    (for _index_2 (range (* _renderrange -1) _renderrange) ; y
      (bind _returnvalue (Game|SpawnActorfromClass "/Game/Blueprints/Items/World/BP_Chunk.BP_Chunk_C" (Math|Transform|MakeTransform (Math|Vector|MakeVector (Math|Conversions|ToFloat(Integer) (* _index (* (Variables|Default|Tile|GetTileSize) 100))) (Math|Conversions|ToFloat(Integer) (* _index_2 (* (Variables|Default|Tile|GetTileSize) 100))) 0.0) "0, 0, 0" "1,1,1") "Undefined" 0 0))
      (Utilities|Array|Add (Variables|Info|GetBlockCoordinates) (Utilities|Struct|MakeS_BlockCoordinates (Math|Vector2D|MakeVector2D (.X (Math|Vector|BreakVector (Transformation|GetActorLocation _returnvalue))) (.Y (Math|Vector|BreakVector (Transformation|GetActorLocation _returnvalue)))) _returnvalue)))))

(fn UpdatePosition
  (bind _output_get (Variables|Info|SetCharacterPosition (Transformation|GetActorLocation (Game|Player|GetPlayerPawn 0))))
  (if (or (!= (Variables|TEST|GetChunkX) (Math|Float|Floor (/ (.X (Math|Vector|BreakVector _output_get)) (Math|Conversions|ToFloat(Integer) (Variables|TEST|GetChunkSize))))) (!= (Variables|TEST|GetChunkX) (Math|Float|Floor (/ (.Y (Math|Vector|BreakVector _output_get)) (Math|Conversions|ToFloat(Integer) (Variables|TEST|GetChunkSize))))))
    (Variables|TEST|SetChunkX (Math|Float|Floor (/ (.X (Math|Vector|BreakVector _output_get)) (Math|Conversions|ToFloat(Integer) (Variables|TEST|GetChunkSize)))))
    (Variables|TEST|SetChunkY (Math|Float|Floor (/ (.Y (Math|Vector|BreakVector _output_get)) (Math|Conversions|ToFloat(Integer) (Variables|TEST|GetChunkSize)))))
    (return true)
    (else
      (return false))))