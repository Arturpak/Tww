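; A grass-dirt block that switches between grass and plain dirt materials depending on whether something covers it.
; On BeginPlay or the CheckBlock event, it line-traces down for another grass-dirt block, then up for any blocking hit, which decides the final materials, and plays audio.
; A looping timer repeats the upward trace, so covered blocks turn to dirt and exposed ones regrow grass, with debug traces and print left on.
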(event Custom|CheckBlock
  (CallFunction|CheckBlockLineTrace))

(event EventBeginPlay
  (|CallParentFunction)
  (CallFunction|CheckBlockLineTrace))

(event Collision|EventActorBeginOverlap
  (params (OtherActor :type Actor%20Object%20Reference))
  (|CallParentFunction OtherActor) ; This node is disabled and will not be called.\nDrag off pins to build functionality.
)

(event EventTick
  (params (DeltaSeconds :type Float%20%28single-precision%29))
  (|CallParentFunction DeltaSeconds))

(fn ConstructionScript
  (|CallParentFunction))

(fn CheckBlockLineTrace
  (bind _staticmesh (Variables|Default|GetStaticMesh))
  (bind _staticmesh_2 (Variables|Default|GetStaticMesh))
  (bind _staticmesh_3 (Variables|Default|GetStaticMesh))
  (bind _staticmesh_4 (Variables|Default|GetStaticMesh))
  (bind _returnvalue (Transformation|GetWorldLocation _staticmesh_4))
  (bind _returnvalue_2 (Transformation|GetWorldLocation _staticmesh_3))
  (bind _returnvalue_3 (Math|Vector|GetUpVector _staticmesh_4))
  (Utilities|FlowControl|Sequence
    (:then_0
      ;[0.1719 0.1719 0.1719] Трэйс вниз
      (bind _outhit (Collision|LineTraceByChannel _returnvalue (+ _returnvalue (* (Math|Vector|MakeVector (.x _returnvalue_3) (.y _returnvalue_3) (* (.z _returnvalue_3) -1.0)) 1e+02)) "TraceTypeQuery1" false 0 "ForDuration" true "(R=0.069136,G=1.000000,B=0.000000,A=1.000000)" "(R=1.000000,G=0.007764,B=0.000000,A=1.000000)" 1.0))
      (Utilities|Casting|CastToBP_BlockGrassDirt (.HitActor (Collision|BreakHitResult _outhit)))
      (Rendering|Material|SetMaterial _staticmesh 0 "/Game/Assets/Materials/GrassSide/MI_Dirt.MI_Dirt")
      (Rendering|Material|SetMaterial _staticmesh 1 "/Game/Assets/Materials/GrassSide/MI_Dirt.MI_Dirt"))
    (:then_1
      ;[0.1719 0.1719 0.1719] Трэйс вверх
      (bind _outhit_2 (Collision|LineTraceByChannel _returnvalue_2 (+ _returnvalue_2 (* (Math|Vector|GetUpVector _staticmesh_3) 1e+02)) "TraceTypeQuery1" false 0 "ForDuration" true "(R=0.069136,G=1.000000,B=0.000000,A=1.000000)" "(R=1.000000,G=0.007764,B=0.000000,A=1.000000)" 1.0))
      (if (.bBlockingHit (Collision|BreakHitResult _outhit_2))
        (Rendering|Material|SetMaterial _staticmesh_2 0 "/Game/Assets/Materials/GrassSide/MI_Dirt.MI_Dirt")
        (Rendering|Material|SetMaterial _staticmesh_2 1 "/Game/Assets/Materials/GrassSide/MI_Dirt.MI_Dirt")
        (else
          (Rendering|Material|SetMaterial _staticmesh_2 0 "/Game/Assets/Materials/GrassSide/MI_GrassDefault_Up.MI_GrassDefault_Up")
          (Rendering|Material|SetMaterial _staticmesh_2 1 "/Game/Assets/Materials/GrassSide/MI_GrassDirt.MI_GrassDirt")))
      (Utilities|Time|SetTimerbyFunctionName 0 "SetTextureDirt>Grass" 6.0 true)))
  (Audio|Components|Audio|Play (Variables|Default|GetAudio) 0.0))

(fn SetTextureDirt>Grass
  (bind _staticmesh (Variables|Default|GetStaticMesh))
  (bind _staticmesh_2 (Variables|Default|GetStaticMesh))
  (bind _returnvalue (Transformation|GetWorldLocation _staticmesh))
  (bind _outhit (Collision|LineTraceByChannel _returnvalue (+ _returnvalue (* (Math|Vector|GetUpVector _staticmesh) 1e+02)) "TraceTypeQuery1" false 0 "ForDuration" true "(R=0.069136,G=1.000000,B=0.000000,A=1.000000)" "(R=1.000000,G=0.007764,B=0.000000,A=1.000000)" 1.0))
  (if (.bBlockingHit (Collision|BreakHitResult _outhit))
    (Rendering|Material|SetMaterial _staticmesh_2 0 "/Game/Assets/Materials/GrassSide/MI_Dirt.MI_Dirt")
    (Rendering|Material|SetMaterial _staticmesh_2 1 "/Game/Assets/Materials/GrassSide/MI_Dirt.MI_Dirt")
    (CallFunction|PrintText "ПРОВЕРКА НА ЗЕМЛЮ" "(R=1.000000,G=0.339252,B=0.087070,A=1.000000)" 2.0)
    (else
      (Rendering|Material|SetMaterial _staticmesh_2 0 "/Game/Assets/Materials/GrassSide/MI_GrassDefault_Up.MI_GrassDefault_Up")
      (Rendering|Material|SetMaterial _staticmesh_2 1 "/Game/Assets/Materials/GrassSide/MI_GrassDirt.MI_GrassDirt"))))