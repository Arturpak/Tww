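; Base block actor whose look and item drop are driven by its ItemStructure data.
; The construction script calls Init to apply the mesh and three material slots from that struct.
; SpawnItem and the SpawnIII event optionally spawn a pickup-class actor at the block's transform and pass it the struct, with SpawnIII setting the player controller as owner.
; Destroyed and PlaySoundEvent play 2D sounds.
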(event Custom|Play%20Sound%20Event
  (Audio|PlaySound2D (Variables|Default|GetPlaySoundEvent) 1.0 1.0 0.0 0 0))

(event Custom|SpawnIII
  (if (Variables|Default|GetSpawn?)
    (bind _returnvalue (Game|SpawnActorfromClass (Variables|Default|GetDestroyedSpawnItem%20) (Transformation|GetActorTransform) "Undefined" (Game|GetPlayerController 0) 0))
    (Class|BPIRemoveBlock|ItemParameters(Message) _returnvalue (Variables|Default|GetItemStructure))))

(event EventDestroyed
  (Audio|PlaySound2D (Variables|Default|GetSoundDestroy) 1.0 1.0 0.0 0 0))

(fn ConstructionScript
  (CallFunction|Init))

(fn Init
  (bind _staticmesh (Variables|Default|GetStaticMesh))
  (bind _itemstructure (Variables|Default|GetItemStructure))
  (bind (_description _type _staticmesh_2 _materials) (Utilities|Struct|BreakS_ItemParameters _itemstructure))
  (bind (_index0 _index1 _index2) (Utilities|Struct|BreakS_BlockMaterial _materials))
  (Components|StaticMesh|SetStaticMesh _staticmesh _staticmesh_2)
  (Rendering|Material|SetMaterial _staticmesh 0 _index0)
  (Rendering|Material|SetMaterial _staticmesh 1 _index1)
  (Rendering|Material|SetMaterial _staticmesh 2 _index2))

(fn SpawnItem
  (if (Variables|Default|GetSpawn?)
    (bind _returnvalue (Game|SpawnActorfromClass (Variables|Default|GetDestroyedSpawnItem%20) (Transformation|GetActorTransform) "Undefined" 0 0))
    (Class|BPIRemoveBlock|ItemParameters(Message) _returnvalue (Variables|Default|GetItemStructure))))