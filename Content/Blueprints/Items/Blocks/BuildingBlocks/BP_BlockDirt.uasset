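; BP_BlockDirt is a dirt building block that turns its appearance to grass when nothing is above it.
; A looping timer, started by function name on BeginPlay, runs a Visibility line trace upward from the mesh every few seconds.
; When the trace finds no blocking hit, two material slots switch to grass materials, with no path back to dirt.
; The trace leaves debug drawing enabled.
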(event EventBeginPlay
  (|CallParentFunction)
  (Utilities|Time|SetTimerbyFunctionName 0 "Trace line Up Dirt>Grass" 3.0 true))

(event Collision|EventActorBeginOverlap
  (params (OtherActor :type Actor%20Object%20Reference))
  (|CallParentFunction OtherActor) ; This node is disabled and will not be called.\nDrag off pins to build functionality.
)

(event EventTick
  (params (DeltaSeconds :type Float%20%28single-precision%29))
  (|CallParentFunction DeltaSeconds) ; This node is disabled and will not be called.\nDrag off pins to build functionality.
)

(fn ConstructionScript
  (|CallParentFunction))

(fn TraceLineUpDirt>Grass
  (bind _staticmesh (Variables|Default|GetStaticMesh))
  (bind _staticmesh_2 (Variables|Default|GetStaticMesh))
  (bind _returnvalue (Transformation|GetWorldLocation _staticmesh_2))
  (bind _outhit (Collision|LineTraceByChannel _returnvalue (+ _returnvalue (* (Math|Vector|GetUpVector _staticmesh_2) 1e+02)) "TraceTypeQuery1" false 0 "ForDuration" true "(R=0.069136,G=1.000000,B=0.000000,A=1.000000)" "(R=1.000000,G=0.007764,B=0.000000,A=1.000000)" 6.0))
  (if (not (.bBlockingHit (Collision|BreakHitResult _outhit)))
    (Rendering|Material|SetMaterial _staticmesh 0 "/Game/Assets/Materials/GrassSide/MI_GrassDefault_Up.MI_GrassDefault_Up")
    (Rendering|Material|SetMaterial _staticmesh 1 "/Game/Assets/Materials/GrassSide/MI_GrassDirt.MI_GrassDirt")))