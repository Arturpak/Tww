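; BP_MagicStone1 is a stone half-block that merges with another of its kind beneath it into a full block.
; On BeginPlay a short debug downward trace looks for that block; on a hit it destroys it, swaps to the Block mesh, shifts up and clears Poly.
; While Poly is set, Box overlap by FirstPersonCharacter plays a timeline, then offsets the character vertically once it finishes.
; The dirt-to-grass trace function is an unconnected stub.
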(event OnComponentBeginOverlap(Box)
  (params (OverlappedComponent :type Primitive%20Component%20Object%20Reference) (OtherActor :type Actor%20Object%20Reference) (OtherComp :type Primitive%20Component%20Object%20Reference) (OtherBodyIndex :type Integer) (bFromSweep :type Boolean) (SweepResult :type Hit%20Result%20Structure%20%28by%20ref%29))
  (bind _asfirst_person_character (Utilities|Casting|CastToFirstPersonCharacter OtherActor))
  (if (Variables|Default|GetPoly?)
    (bind _newtrack_0 (Timeline|Timeline_0 PlayFromStart)
      (:Finished
        (Transformation|AddActorWorldOffset _asfirst_person_character (Math|Vector|MakeVector 0.0 0.0 _newtrack_0))))))

(event EventBeginPlay
  (bind _staticmesh (Variables|Default|GetStaticMesh))
  (bind _staticmesh_2 (Variables|Default|GetStaticMesh))
  (bind _staticmesh_3 (Variables|Default|GetStaticMesh))
  (bind _returnvalue (Transformation|GetWorldLocation _staticmesh))
  (bind _returnvalue_2 (Math|Vector|GetUpVector _staticmesh))
  (bind _returnvalue_3 (Transformation|GetWorldLocation _staticmesh_3))
  (bind (_x _y _z) (Math|Vector|BreakVector _returnvalue_3))
  (|CallParentFunction)
  (bind _outhit (Collision|LineTraceByChannel _returnvalue (+ _returnvalue (Math|Vector|MakeVector (.x _returnvalue_2) (.y _returnvalue_2) (* (.z _returnvalue_2) -1.0))) "TraceTypeQuery1" false 0 "ForDuration" true "(R=0.069136,G=1.000000,B=0.000000,A=1.000000)" "(R=1.000000,G=0.007764,B=0.000000,A=1.000000)" 1.0))
  (bind _asbp_magic_stone_1 (Utilities|Casting|CastToBP_MagicStone1 (.HitActor (Collision|BreakHitResult _outhit)))
    (:then
      (CallFunction|PrintText "Снизу полублок" "(R=1.000000,G=0.339252,B=0.087070,A=1.000000)" 2.0)
      (Actor|DestroyActor _asbp_magic_stone_1)
      (Components|StaticMesh|SetStaticMesh _staticmesh_2 "/Game/Assets/Meshes/Blocks/Block.Block")
      (Transformation|SetWorldTransform _staticmesh_2 (Math|Transform|MakeTransform (Math|Vector|MakeVector _x _y (+ _z 25.0))) false false)
      (Variables|Default|SetPoly? false))
    (:CastFailed
      (CallFunction|PrintText "Всё норм" "(R=1.000000,G=0.339252,B=0.087070,A=1.000000)" 2.0))))

(event Collision|EventActorBeginOverlap
  (params (OtherActor :type Actor%20Object%20Reference))
  (|CallParentFunction OtherActor) ; This node is disabled and will not be called.\nDrag off pins to build functionality.
)

(event EventTick
  (params (DeltaSeconds :type Float%20%28single-precision%29))
  (|CallParentFunction DeltaSeconds) ; This node is disabled and will not be called.\nDrag off pins to build functionality.
)

(fn ConstructionScript
  (|CallParentFunction))

(fn TraceLineUpDirt>Grass)